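; Desktop PC player character built on VR components, letting motion controllers follow the camera with mouse-style look input.
; BeginPlay attaches both motion controllers to the replicated VR camera, keeping relative transforms, and removes the camera as their tick prerequisite.
; It also adds the PC Enhanced Input mapping context for player 0.
; The look action drives controller yaw and pitch, with the vertical axis inverted.
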(event `self.ReceiveBeginPlay`
  (bind _vrreplicatedcamera (`self.VRReplicatedCamera`))
  (bind _returnvalue (pcsubsystem `EnhancedInputLocalPlayerSubsystem` (`GameplayStatics.GetPlayerController` 0)))
  (`parent.ReceiveBeginPlay`)
  (`SceneComponent.K2_AttachToComponent` (`self.LeftMotionController`) _vrreplicatedcamera "None" "KeepRelative" "KeepRelative" "KeepRelative" true)
  (`SceneComponent.K2_AttachToComponent` (`self.RightMotionController`) _vrreplicatedcamera "None" "KeepRelative" "KeepRelative" "KeepRelative" true)
  (`ActorComponent.RemoveTickPrerequisiteComponent` (`self.LeftMotionController`) (`self.VRReplicatedCamera`))
  (`ActorComponent.RemoveTickPrerequisiteComponent` (`self.RightMotionController`) (`self.VRReplicatedCamera`))
  (`/Engine/EditorBlueprintResources/StandardMacros.IsValid` _returnvalue
    (:`Is Valid`
      (`EnhancedInputSubsystemInterface.AddMappingContext` _returnvalue "/Game/Input/IMC_PCInputContext.IMC_PCInputContext" 0 (struct)))))

(event `EnhancedInput|/Game/Input/IA_PCLook`
  (params (ActionValue :type "Vector2D Structure") (ElapsedSeconds :type "Float (double-precision)") (TriggeredSeconds :type "Float (double-precision)") (InputAction :type "InputAction Object Reference" :default "/Game/Input/IA_PCLook.IA_PCLook"))
  (:`Triggered`
    (`self.AddControllerYawInput` ActionValue_X)
    (`self.AddControllerPitchInput` (* ActionValue_Y -1.0))))

(fn `UserConstructionScript`
  (`parent.UserConstructionScript`))
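; BP_Planet is a planet actor that spins on its axis and orbits a referenced sun actor.
; Each tick it yaws the mesh and rotates its position around the sun's vertical axis, using its Rotation and Revolution speeds.
; A name label follows the mesh at an offset and turns to face the player camera.
; Highlight and UndoHighlight toggle an overlay material on the mesh and the label's visibility.
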(event `self.ReceiveTick`
  (params (DeltaSeconds :type "Float (single-precision)"))
  (bind _planetmesh (`self.PlanetMesh`))
  (bind _returnvalue (`self.K2_GetActorLocation` (`self.SunReference`)))
  (`SceneComponent.K2_AddLocalRotation` _planetmesh (`KismetMathLibrary.MakeRotator` 0.0 0.0 (* DeltaSeconds (`self.Rotation`))) false false)
  (`self.SetPlanetNameLocationAndRotation` _planetmesh)
  (`self.K2_SetActorLocation` (+ (`KismetMathLibrary.RotateAngleAxis` (- (`self.K2_GetActorLocation`) _returnvalue) (* DeltaSeconds (`self.Revolution`)) (0.0 0.0 1.0)) _returnvalue)))

(event `/Game/Core/BPI_Interact.Highlight`
  (`MeshComponent.SetOverlayMaterial` (`self.PlanetMesh`) "/Game/Material/M_Highlight.M_Highlight")
  (`SceneComponent.SetVisibility` (`self.PlanetName`) true false))

(event `/Game/Core/BPI_Interact.UndoHighlight`
  (`MeshComponent.SetOverlayMaterial` (`self.PlanetMesh`) null)
  (`SceneComponent.SetVisibility` (`self.PlanetName`) false false))

(fn `SetPlanetNameLocationAndRotation`
  (params (PlanetMesh :type "GrippableStaticMeshComponent Object Reference"))
  (bind _planetname (`self.PlanetName`))
  (`SceneComponent.K2_SetWorldLocation` _planetname (+ (`SceneComponent.K2_GetComponentLocation` PlanetMesh) (`self.PlanetNameLocation`)) false false)
  (`SceneComponent.K2_SetWorldRotation` _planetname (`KismetMathLibrary.FindLookAtRotation` (`SceneComponent.K2_GetComponentLocation` (`self.PlanetName`)) (`SceneComponent.K2_GetComponentLocation` (`PlayerCameraManager.TransformComponent` (`GameplayStatics.GetPlayerCameraManager` 0)))) false false)
  (return))

(fn `UserConstructionScript`)